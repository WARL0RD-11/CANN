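; GA_Combo1 is a Gameplay Ability for the first attack in the main character's combo.
; On activation it commits, points the "Attack1" motion warp target at the first BP_Enemy found, with yaw flipped 180 degrees, and plays a sped-up montage.
; Gameplay events for the combo window add and remove a loose ComboWindowOpen tag on the avatar, and the window-end event ends the ability.
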(event Ability|EventActivateAbility
  (Ability|CommitAbility)
  (bind _asbp_main_character (Utilities|Casting|CastToBP_MainCharacter (Game|Player|GetPlayerPawn 0)))
  (bind _outactors (Actor|GetAllActorsOfClass "/Game/Blueprints/Enemy/BP_Enemy.BP_Enemy_C"))
  (Class|MotionWarpingComponent|AddorUpdateWarpTarget (Variables|/Game/Blueprints/Character/BP_MainCharacter.BP_MainCharacter_C|GetMotionWarping _asbp_main_character) (Utilities|Struct|MakeMotionWarpingTarget "Attack1" (Transformation|GetActorLocation (Utilities|Array|Get(acopy) _outactors)) (Math|Rotator|MakeRotator (.roll (Transformation|GetActorRotation (Utilities|Array|Get(acopy) _outactors))) (.pitch (Transformation|GetActorRotation (Utilities|Array|Get(acopy) _outactors))) (+ (.yaw (Transformation|GetActorRotation (Utilities|Array|Get(acopy) _outactors))) 1.8e+02)) 0 "None" false "0.000000,0.000000,0.000000" "0.000000,0.000000,0.000000"))
  (|PlayMontageandWaitProxy "None" (Variables|Default|GetMontage%20to%20Play) 1.5 "None" true 1.0 0.0 false
    (:then
      (Ability|Tasks|WaitGameplayEvent "(TagName=\"Event.ComboWindowOpen\")" 0
        (:then
          (Ability|Tasks|WaitGameplayEvent "(TagName=\"Event.ComboWindowEnd\")" 0
            (:EventReceived
              (Development|PrintString "Combo 1 Window Closed")
              (Ability|GameplayEffect|RemoveLooseGameplayTags (Ability|GetAvatarActorfromActorInfo) (Variables|Default|GetComboWindowOpenTag))
              (Ability|EndAbility))))
        (:EventReceived
          (Development|PrintString "Combo1 Window Open")
          (Ability|GameplayEffect|AddLooseGameplayTags (Ability|GetAvatarActorfromActorInfo) (Variables|Default|GetComboWindowOpenTag)))))))

(event Ability|EventOnEndAbility
  (params (bWasCancelled :type Boolean))
  (Development|PrintString "Combo1 ended"))