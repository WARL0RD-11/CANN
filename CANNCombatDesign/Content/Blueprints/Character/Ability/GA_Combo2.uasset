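; GA_Combo2 is a Gameplay Ability for the second attack in the main character's combo.
; It sets the "Attack2" motion warp target from the first BP_Enemy found, using its location and negated rotation, then plays a sped-up montage.
; Gameplay events open the combo window, swapping Combo1Tag for ComboWindowTag, and close it, removing that tag and ending the ability.
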(event Ability|EventActivateAbility
  (Ability|CommitAbility)
  (bind _asbp_main_character (Utilities|Casting|CastToBP_MainCharacter (Game|Player|GetPlayerPawn 0)))
  (bind _outactors (Actor|GetAllActorsOfClass "/Game/Blueprints/Enemy/BP_Enemy.BP_Enemy_C"))
  (Class|MotionWarpingComponent|AddorUpdateWarpTarget (Variables|/Game/Blueprints/Character/BP_MainCharacter.BP_MainCharacter_C|GetMotionWarping _asbp_main_character) (Utilities|Struct|MakeMotionWarpingTarget "Attack2" (Transformation|GetActorLocation (Utilities|Array|Get(acopy) _outactors)) (* (Transformation|GetActorRotation (Utilities|Array|Get(acopy) _outactors)) -1.0) 0 "None" false "0.000000,0.000000,0.000000" "0.000000,0.000000,0.000000"))
  (|PlayMontageandWaitProxy "None" (Variables|Default|GetMontage%20to%20Play) 1.5 "None" true 1.0 0.0 false
    (:then
      (Ability|Tasks|WaitGameplayEvent "(TagName=\"Event.ComboWindowOpen\")" 0
        (:then
          (Ability|Tasks|WaitGameplayEvent "(TagName=\"Event.ComboWindowEnd\")" 0
            (:EventReceived
              (Development|PrintString "Combo2 Window Closed")
              (Ability|GameplayEffect|RemoveLooseGameplayTags (Ability|GetAvatarActorfromActorInfo) (Variables|Default|GetComboWindowTag))
              (Ability|EndAbility))))
        (:EventReceived
          (Development|PrintString "Combo2 Window Open")
          (Ability|GameplayEffect|RemoveLooseGameplayTags (Ability|GetAvatarActorfromActorInfo) (Variables|Default|GetCombo1Tag))
          (Ability|GameplayEffect|AddLooseGameplayTags (Ability|GetAvatarActorfromActorInfo) (Variables|Default|GetComboWindowTag)))))))

(event Ability|EventOnEndAbility
  (params (bWasCancelled :type Boolean))
  (Development|PrintString "Combo2 ended"))