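; BP_Sword is a sword pickup that attaches to the player character's back when picked up.
; PickingUp caches the player as BP_MainCharacter, waits a very brief delay, runs WeaponSlot and prints a debug message.
; For slot 0, WeaponSlot snaps the ItemType component to the SwordInBack socket and stores it as the character's Sword.
; The construction script applies the configured skeletal mesh to ItemType.
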(event EventPickingUp
  (bind _asbp_main_character (Utilities|Casting|CastToBP_MainCharacter (Game|GetPlayerCharacter 0)))
  (Variables|Default|SetMainChar _asbp_main_character)
  (Utilities|FlowControl|Delay 0.002)
  (Utilities|WeaponSlot
    (:OUT
      (Development|PrintString "W picked Up"))))

(fn ConstructionScript
  (Components|SkeletalMesh|SetSkeletalMeshAsset (Variables|Default|GetItemType) (Variables|Default|GetSkeletalMesh)))