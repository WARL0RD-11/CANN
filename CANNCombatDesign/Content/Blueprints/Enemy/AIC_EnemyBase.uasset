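; Base AI controller for enemies that runs their shared behavior tree and targets the player.
; On possess, it waits briefly, starts BT_EnemyBase, then stores the first player's character in the blackboard as the attack target.
; Two helper functions write an E_EnemyState value to the blackboard to mark the enemy as dead or frozen.
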(event EventPossess
  (params (PossessedPawn :type Pawn%20Object%20Reference))
  (Utilities|FlowControl|Delay 0.2)
  (AI|RunBehaviorTree "/Game/Blueprints/Enemy/BT_EnemyBase.BT_EnemyBase")
  (AI|Components|Blackboard|SetValueasObject (Variables|Default|GetBlackboard) (Variables|Default|GetAttackTargetKeyName) (Game|GetPlayerCharacter 0)))

(fn ConstructionScript)

(fn SetStateasDead
  (AI|Components|Blackboard|SetValueasEnum (Variables|Default|GetBlackboard) (Variables|Default|GetStateKeyName) (Utilities|Enum|LiteralenumE_EnemyState "NewEnumerator1")))

(fn SetStateasFrozen
  (AI|Components|Blackboard|SetValueasEnum (Variables|Default|GetBlackboard) (Variables|Default|GetStateKeyName) (Utilities|Enum|LiteralenumE_EnemyState "NewEnumerator0")))